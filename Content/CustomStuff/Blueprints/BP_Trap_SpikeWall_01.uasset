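; BP_Trap_SpikeWall_01 is a spike wall trap that swings on a hinge when the ThirdPersonCharacter enters or leaves its trigger box.
; Begin overlap plays an activation timeline that drives the Hinge's relative yaw, and end overlap plays a separate deactivation timeline on the same yaw.
; When either timeline finishes, it prints a debug message and plays a 2D click sound.
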(event OnComponentBeginOverlap(TriggerBox)
  (params (OverlappedComponent :type Primitive%20Component%20Object%20Reference) (OtherActor :type Actor%20Object%20Reference) (OtherComp :type Primitive%20Component%20Object%20Reference) (OtherBodyIndex :type Integer) (bFromSweep :type Boolean) (SweepResult :type Hit%20Result%20Structure%20%28by%20ref%29))
  (Utilities|Casting|CastToThirdPersonCharacter OtherActor)
  (bind _trap_rotation (Timeline|TrapActivationRotation PlayFromStart)
    (:Update
      (Transformation|SetRelativeRotation (Variables|Default|GetHinge) (Math|Rotator|MakeRotator 0.0 0.0 _trap_rotation) false false))
    (:Finished
      (Development|PrintString "Spike Wall Trap Activated")
      (Audio|PlaySound2D "/Engine/VREditor/Sounds/VR_click1.VR_click1" 1.0 1.0 0.0 0 0))))

(event OnComponentEndOverlap(TriggerBox)
  (params (OverlappedComponent :type Primitive%20Component%20Object%20Reference) (OtherActor :type Actor%20Object%20Reference) (OtherComp :type Primitive%20Component%20Object%20Reference) (OtherBodyIndex :type Integer))
  (Utilities|Casting|CastToThirdPersonCharacter OtherActor)
  (bind _trap_rotation (Timeline|TrapDeactivatingRotation PlayFromStart)
    (:Update
      (Transformation|SetRelativeRotation (Variables|Default|GetHinge) (Math|Rotator|MakeRotator 0.0 0.0 _trap_rotation) false false))
    (:Finished
      (Development|PrintString "Spike Wall Trap deactivated")
      (Audio|PlaySound2D "/Engine/VREditor/Sounds/VR_click3.VR_click3" 1.0 1.0 0.0 0 0))))

(fn ConstructionScript)